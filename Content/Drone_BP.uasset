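; Drone pawn flown from the keyboard through a FloatingPawnMovement component.
; E and Q set vertical movement, W and S handle ForwardForce, and A and D set a rotation delta, with releases resetting each.
; Tick feeds MoveVector plus the forward vector offset by ForwardForce into movement input and applies the rotation.
; ForwardForce is added rather than multiplied, and pressing W leaves it unchanged.
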(event `Key|E`
  (params (Key :type "Key Structure"))
  (:`Pressed`
    (set `self.MoveVector` (0.0 0.0 1.0)))
  (:`Released`
    (set `self.MoveVector` (0.0 0.0 0.0) :!label _label)))

(event `self.ReceiveTick`
  (params (DeltaSeconds :type "Float (single-precision)"))
  (`PawnMovementComponent.AddInputVector` (`self.FloatingPawnMovement`) (+ (`self.MoveVector`) (+ (`self.GetActorForwardVector`) (`self.ForwardForce`))) false)
  (`self.K2_AddActorWorldRotation` (`self.Rotator`)))

(event `Key|Q`
  (params (Key :type "Key Structure"))
  (:`Pressed`
    (set `self.MoveVector` (0.0 0.0 -1.0)))
  (:`Released`
    (goto _label)))

(event `Key|W`
  (params (Key :type "Key Structure"))
  (:`Pressed`
    (set `self.ForwardForce` (`self.ForwardForce`)))
  (:`Released`
    (set `self.ForwardForce` 0.0 :!label _label_2)))

(event `Key|S`
  (params (Key :type "Key Structure"))
  (:`Pressed`
    (set `self.ForwardForce` (+ (`self.ForwardForce`) -1.0)))
  (:`Released`
    (goto _label_2)))

(event `Key|A`
  (params (Key :type "Key Structure"))
  (:`Pressed`
    (set `self.Rotator` (`KismetMathLibrary.MakeRotator` 0.0 0.0 (+ (`self.RotateSpeed`) -1.0))))
  (:`Released`
    (set `self.Rotator` (`KismetMathLibrary.MakeRotator` 0.0))))

(event `Key|D`
  (params (Key :type "Key Structure"))
  (:`Pressed`
    (set `self.Rotator` (`KismetMathLibrary.MakeRotator` 0.0 0.0 (`self.RotateSpeed`))))
  (:`Released`
    (set `self.Rotator` (`KismetMathLibrary.MakeRotator` 0.0))))

(fn `UserConstructionScript`)